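; Player-controlled tilting table for a ball game, hosting the current level as a child actor.
; Enhanced Input nudges roll and pitch in fixed steps, while events spawn balls or destroy the ball, level the table and load the next level.
; Tick checks for zero lives, then inserts the run into saved rankings by level and time fields, saves, shows the GameOver widget and pauses.
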(event Custom|DropBall
  (params (Location :type Vector))
  (Game|SpawnActorfromClass "/Game/Blueprints/BP_TheBall.BP_TheBall_C" (Math|Transform|MakeTransform Location "0, 0, 0" "1.000000,1.000000,1.000000") "Undefined" "MultiplyWithRoot" 0 0))

(event Custom|NextLevel
  (params (TheBall :type Actor%20Object%20Reference))
  (Actor|DestroyActor TheBall)
  (Transformation|SetActorRotation "0, 0, 0")
  (Variables|Default|SetCurrentLevel (+ (Variables|Default|GetCurrentLevel) 1))
  (ChildActorComponent|SetChildActorClass (Variables|Default|GetCurrentLevelOn) (Utilities|Array|Get(acopy) (Variables|Default|GetLevels) (- (Variables|Default|GetCurrentLevel) 1))))

(event Input|EnhancedActionEvents|EnhancedInputActionIA_LeftRight
  (params (ActionValue :type Float%20%28double-precision%29) (ElapsedSeconds :type Float%20%28double-precision%29) (TriggeredSeconds :type Float%20%28double-precision%29) (InputAction :type Input%20Action%20Object%20Reference :default "/Game/Inputs/IA_LeftRight.IA_LeftRight"))
  (bind _returnvalue (Transformation|GetActorRotation))
  (bind _returnvalue_2 (Transformation|GetActorRotation))
  (if (< ActionValue 0.0)
    (Transformation|SetActorRotation (Math|Rotator|MakeRotator (+ (.roll _returnvalue) -0.25) (.pitch _returnvalue) 0.0))
    (else
      (Transformation|SetActorRotation (Math|Rotator|MakeRotator (+ (.roll _returnvalue_2) 0.25) (.pitch _returnvalue_2) 0.0)))))

(event Input|EnhancedActionEvents|EnhancedInputActionIA_UpDown
  (params (ActionValue :type Float%20%28double-precision%29) (ElapsedSeconds :type Float%20%28double-precision%29) (TriggeredSeconds :type Float%20%28double-precision%29) (InputAction :type Input%20Action%20Object%20Reference :default "/Game/Inputs/IA_UpDown.IA_UpDown"))
  (bind _returnvalue (Transformation|GetActorRotation))
  (bind _returnvalue_2 (Transformation|GetActorRotation))
  (if (< ActionValue 0.0)
    (Transformation|SetActorRotation (Math|Rotator|MakeRotator (.roll _returnvalue) (+ (.pitch _returnvalue) 0.25) 0.0))
    (else
      (Transformation|SetActorRotation (Math|Rotator|MakeRotator (.roll _returnvalue_2) (+ (.pitch _returnvalue_2) -0.25) 0.0)))))

(event EventBeginPlay
  (CallFunction|SetupInput)
  (CallFunction|InitializeVariables)
  (ChildActorComponent|SetChildActorClass (Variables|Default|GetCurrentLevelOn) (Utilities|Array|Get(acopy) (Variables|Default|GetLevels))))

(event EventTick
  (params (DeltaSeconds :type Float%20%28single-precision%29))
  (CallFunction|CheckGameOver))

(fn ConstructionScript)

(fn SetupInput
  (bind _asbp_my_controller (Utilities|Casting|CastToBP_MyController (Pawn|GetController)))
  (Input|AddMappingContext (PlayerController|LocalPlayerSubsystems|GetEnhancedInputLocalPlayerSubsystem _asbp_my_controller) "/Game/Inputs/IMC_Inputs.IMC_Inputs" 0 "(bIgnoreAllPressedKeysUntilRelease=True,bForceImmediately=False,bNotifyUserSettings=False)"))

(fn InitializeVariables
  (Variables|Default|SetLives 3)
  (Variables|Default|SetCurrentLevel 1)
  (bind _asglobal_game_variables (Utilities|Casting|CastToGlobalGameVariables (Game|GetGameInstance)))
  (Variables|Default|SetGlobals _asglobal_game_variables)
  (bind _returnvalue (SaveGame|LoadGamefromSlot "TheSave"))
  (bind _asmain_save (Utilities|Casting|CastToMainSave _returnvalue))
  (Variables|Default|SetTheSave _asmain_save))

(fn CheckGameOver
  (if (<= (Variables|Default|GetLives) 0)
    (bind _index (Utilities|FlowControl|ForLoopwithBreak 0 (- (Utilities|Array|Length (Variables|/Game/Blueprints/MainSave.MainSave_C|GetSLevels (Variables|Default|GetTheSave))) 1) :!label _label)
      (:LoopBody
        (if (> (Variables|Default|GetCurrentLevel) (Utilities|Array|Get(acopy) (Variables|/Game/Blueprints/MainSave.MainSave_C|GetSLevels (Variables|Default|GetTheSave)) _index))
          (Utilities|Array|Insert (Variables|/Game/Blueprints/MainSave.MainSave_C|GetSLevels (Variables|Default|GetTheSave)) (Variables|Default|GetCurrentLevel) _index :!label _label_2)
          (Utilities|Array|Insert (Variables|/Game/Blueprints/MainSave.MainSave_C|GetSNames (Variables|Default|GetTheSave)) (Variables|/Game/Blueprints/GlobalGameVariables.GlobalGameVariables_C|GetGPlayerName (Variables|Default|GetGlobals)) _index)
          (Utilities|Array|Insert (Variables|/Game/Blueprints/MainSave.MainSave_C|GetSMinutes (Variables|Default|GetTheSave)) (Variables|/Game/Blueprints/GlobalGameVariables.GlobalGameVariables_C|GetGMinutes (Variables|Default|GetGlobals)) _index)
          (Utilities|Array|Insert (Variables|/Game/Blueprints/MainSave.MainSave_C|GetSSeconds (Variables|Default|GetTheSave)) (Variables|/Game/Blueprints/GlobalGameVariables.GlobalGameVariables_C|GetGSeconds (Variables|Default|GetGlobals)) _index)
          (Utilities|Array|Insert (Variables|/Game/Blueprints/MainSave.MainSave_C|GetSMiliSeconds (Variables|Default|GetTheSave)) (Variables|/Game/Blueprints/GlobalGameVariables.GlobalGameVariables_C|GetGMiliSeconds (Variables|Default|GetGlobals)) _index)
          (goto _label Break)
          (elif (< (Variables|/Game/Blueprints/GlobalGameVariables.GlobalGameVariables_C|GetGMinutes (Variables|Default|GetGlobals)) (Utilities|Array|Get(acopy) (Variables|/Game/Blueprints/MainSave.MainSave_C|GetSMinutes (Variables|Default|GetTheSave)) _index))
            (goto _label_2)
            (elif (< (Variables|/Game/Blueprints/GlobalGameVariables.GlobalGameVariables_C|GetGSeconds (Variables|Default|GetGlobals)) (Utilities|Array|Get(acopy) (Variables|/Game/Blueprints/MainSave.MainSave_C|GetSSeconds (Variables|Default|GetTheSave)) _index))
              (goto _label_2)
              (elif (< (Variables|/Game/Blueprints/GlobalGameVariables.GlobalGameVariables_C|GetGMiliSeconds (Variables|Default|GetGlobals)) (Utilities|Array|Get(acopy) (Variables|/Game/Blueprints/MainSave.MainSave_C|GetSMiliSeconds (Variables|Default|GetTheSave)) _index))
                (goto _label_2))))))
      (:Completed
        (SaveGame|SaveGametoSlot (Variables|Default|GetTheSave) "TheSave")
        (bind _returnvalue (UserInterface|CreateWidget "/Game/UI/GameOver.GameOver_C"))
        (UserInterface|Viewport|AddtoViewport _returnvalue 0)
        (Game|SetGamePaused true)))))