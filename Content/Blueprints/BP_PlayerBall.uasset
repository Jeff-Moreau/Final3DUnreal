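; BP_PlayerBall is the player ball Blueprint, handling the ball's rolling and drop sounds.
; Each Tick, it starts the rolling sound if the Ball component has any velocity and it is not already playing, and stops it at exactly zero velocity.
; A HitOnce flag, armed on BeginPlay, limits the drop sound to the first blocking hit.
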(event EventBeginPlay
  (Variables|Default|SetHitOnce true))

(event Collision|EventActorBeginOverlap
  (params (OtherActor :type Actor%20Object%20Reference)))

(event EventTick
  (params (DeltaSeconds :type Float%20%28single-precision%29))
  (if (Utilities|Operators|NotEqual(!=) :A (Transformation|GetComponentVelocity (Variables|Default|GetBall)))
    (if (not (Audio|Components|Audio|IsPlaying (Variables|Default|GetBallRolling)))
      (Audio|Components|Audio|Play (Variables|Default|GetBallRolling) 0.0))
    (else
      (Audio|Components|Audio|Stop (Variables|Default|GetBallRolling)))))

(event Collision|EventHit
  (params (MyComp :type Primitive%20Component%20Object%20Reference) (Other :type Actor%20Object%20Reference) (OtherComp :type Primitive%20Component%20Object%20Reference) (bSelfMoved :type Boolean) (HitLocation :type Vector :default "0, 0, 0") (HitNormal :type Vector :default "0, 0, 0") (NormalImpulse :type Vector :default "0, 0, 0") (Hit :type Hit%20Result%20Structure%20%28by%20ref%29))
  (if (and (Variables|Default|GetHitOnce) (.bBlockingHit (Collision|BreakHitResult Hit)))
    (Variables|Default|SetHitOnce false)
    (if (not (Audio|Components|Audio|IsPlaying (Variables|Default|GetBallDropSound)))
      (Audio|Components|Audio|Play (Variables|Default|GetBallDropSound) 0.0))))

(fn ConstructionScript)