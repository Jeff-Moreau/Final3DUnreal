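; BP_LevelThree is the third level of a tilting-table ball game, dropping the ball at a spawn point on BeginPlay.
; Hitting any of five obstacles resets the table's rotation, returns the ball to the drop point and deducts a life.
; Overlapping the end trigger swaps the goal effect for an explosion, plays a random win sound, then advances the level after short delays.
; The table is the player pawn, and win sounds come from the game instance.
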(event OnComponentBeginOverlap(EndCollision)
  (params (OverlappedComponent :type Primitive%20Component%20Object%20Reference) (OtherActor :type Actor%20Object%20Reference) (OtherComp :type Primitive%20Component%20Object%20Reference) (OtherBodyIndex :type Integer) (bFromSweep :type Boolean) (SweepResult :type Hit%20Result%20Structure%20%28by%20ref%29))
  (Audio|PlaySound2D "/Game/Sounds/SoundFX/bad-explosion-6855.bad-explosion-6855" 1.0 1.0 0.0 0 0)
  (Components|Activation|Deactivate (Variables|Default|GetTheEnd))
  (Components|Activation|Activate (Variables|Default|GetExplosion) false)
  (Utilities|FlowControl|Delay 0.75)
  (Audio|PlaySound2D (.OutItem (Utilities|Array|Random (Variables|/Game/Blueprints/GlobalGameVariables.GlobalGameVariables_C|GetWinSounds (Variables|Default|GetGlobals)))) 1.0 1.0 0.0 0 0)
  (Utilities|FlowControl|Delay 1.0)
  (Default|NextLevel (Variables|Default|GetTheTable) OtherActor))

(event OnComponentHit(ObstacleOne)
  (params (HitComponent :type Primitive%20Component%20Object%20Reference) (OtherActor :type Actor%20Object%20Reference) (OtherComp :type Primitive%20Component%20Object%20Reference) (NormalImpulse :type Vector :default "0, 0, 0") (Hit :type Hit%20Result%20Structure%20%28by%20ref%29))
  (CallFunction|HitBadWall OtherActor))

(event OnComponentHit(ObstacleTwo)
  (params (HitComponent :type Primitive%20Component%20Object%20Reference) (OtherActor :type Actor%20Object%20Reference) (OtherComp :type Primitive%20Component%20Object%20Reference) (NormalImpulse :type Vector :default "0, 0, 0") (Hit :type Hit%20Result%20Structure%20%28by%20ref%29))
  (CallFunction|HitBadWall OtherActor))

(event OnComponentHit(ObstacleThree)
  (params (HitComponent :type Primitive%20Component%20Object%20Reference) (OtherActor :type Actor%20Object%20Reference) (OtherComp :type Primitive%20Component%20Object%20Reference) (NormalImpulse :type Vector :default "0, 0, 0") (Hit :type Hit%20Result%20Structure%20%28by%20ref%29))
  (CallFunction|HitBadWall OtherActor))

(event OnComponentHit(ObstacleFour)
  (params (HitComponent :type Primitive%20Component%20Object%20Reference) (OtherActor :type Actor%20Object%20Reference) (OtherComp :type Primitive%20Component%20Object%20Reference) (NormalImpulse :type Vector :default "0, 0, 0") (Hit :type Hit%20Result%20Structure%20%28by%20ref%29))
  (CallFunction|HitBadWall OtherActor))

(event OnComponentHit(ObstacleFive)
  (params (HitComponent :type Primitive%20Component%20Object%20Reference) (OtherActor :type Actor%20Object%20Reference) (OtherComp :type Primitive%20Component%20Object%20Reference) (NormalImpulse :type Vector :default "0, 0, 0") (Hit :type Hit%20Result%20Structure%20%28by%20ref%29))
  (CallFunction|HitBadWall OtherActor))

(event EventBeginPlay
  (CallFunction|InitializeGlobals)
  (Default|DropBall (Variables|Default|GetTheTable) (Transformation|GetWorldLocation (Variables|Default|GetBallDrop))))

(fn ConstructionScript)

(fn HitBadWall
  (params (InputPin :type Actor%20Object%20Reference))
  (Transformation|SetActorRotation (Variables|Default|GetTheTable))
  (bind _asbp_the_ball (Utilities|Casting|CastToBP_TheBall InputPin))
  (Transformation|SetActorLocation _asbp_the_ball (Transformation|GetWorldLocation (Variables|Default|GetBallDrop)) false false)
  (Variables|/Game/Blueprints/BP_TheTable.BP_TheTable_C|SetLives (Variables|Default|GetTheTable) (- (Variables|/Game/Blueprints/BP_TheTable.BP_TheTable_C|GetLives (Variables|Default|GetTheTable)) 1)))

(fn InitializeGlobals
  (bind _asbp_the_table (Utilities|Casting|CastToBP_TheTable (Game|Player|GetPlayerPawn 0)))
  (Variables|Default|SetTheTable _asbp_the_table)
  (bind _asglobal_game_variables (Utilities|Casting|CastToGlobalGameVariables (Game|GetGameInstance)))
  (Variables|Default|SetGlobals _asglobal_game_variables))