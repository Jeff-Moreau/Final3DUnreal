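; BP_LevelTwo is the second level of a ball game, with a goal trigger and a reset surface for the player ball.
; On BeginPlay it caches the player pawn, a BP_PawnLevelOne, as TheTable.
; A ball overlapping Box is destroyed and TheTable's NextLevel is called.
; A ball hitting Cube4 is moved back to SpawnPoint without sweep or physics teleport.
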(event OnComponentBeginOverlap(Box)
  (params (OverlappedComponent :type Primitive%20Component%20Object%20Reference) (OtherActor :type Actor%20Object%20Reference) (OtherComp :type Primitive%20Component%20Object%20Reference) (OtherBodyIndex :type Integer) (bFromSweep :type Boolean) (SweepResult :type Hit%20Result%20Structure%20%28by%20ref%29))
  (bind _asbp_player_ball (Utilities|Casting|CastToBP_PlayerBall OtherActor))
  (Actor|DestroyActor _asbp_player_ball)
  (Development|PrintString "Next Level")
  (Default|NextLevel (Variables|Default|GetTheTable)))

(event OnComponentHit(Cube4)
  (params (HitComponent :type Primitive%20Component%20Object%20Reference) (OtherActor :type Actor%20Object%20Reference) (OtherComp :type Primitive%20Component%20Object%20Reference) (NormalImpulse :type Vector :default "0, 0, 0") (Hit :type Hit%20Result%20Structure%20%28by%20ref%29))
  (bind _asbp_player_ball (Utilities|Casting|CastToBP_PlayerBall OtherActor))
  (Transformation|SetActorLocation _asbp_player_ball (Transformation|GetWorldLocation (Variables|Default|GetSpawnPoint)) false false))

(event EventBeginPlay
  (bind _asbp_pawn_level_one (Utilities|Casting|CastToBP_PawnLevelOne (Game|Player|GetPlayerPawn 0)))
  (Variables|Default|SetTheTable _asbp_pawn_level_one))

(event Collision|EventActorBeginOverlap
  (params (OtherActor :type Actor%20Object%20Reference)))

(event EventTick
  (params (DeltaSeconds :type Float%20%28single-precision%29)))

(fn ConstructionScript)