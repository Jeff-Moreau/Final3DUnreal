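; Player pawn for a ball game, carrying the level as a child actor and tilting with player input.
; On BeginPlay it adds the Enhanced Input mapping context and spawns a player ball above the origin.
; Left/right and up/down actions nudge the pawn's roll and pitch in small fixed steps by input sign.
; NextLevel levels the pawn, drops a new ball and swaps the child actor class to level two.
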(event Custom|DropBall
  (Game|SpawnActorfromClass "/Game/Blueprints/BP_PlayerBall.BP_PlayerBall_C" (Math|Transform|MakeTransform "0.000000,0.000000,250.000000" "0, 0, 0" "1.000000,1.000000,1.000000") "Undefined" "MultiplyWithRoot" 0 0))

(event Custom|NextLevel
  (Transformation|SetActorRotation "0, 0, 0")
  (CallFunction|DropBall)
  (ChildActorComponent|SetChildActorClass (Variables|Default|GetBP_LevelOne) "/Game/Blueprints/BP_LevelTwo.BP_LevelTwo_C"))

(event Input|EnhancedActionEvents|EnhancedInputActionIA_LeftRight
  (params (ActionValue :type Float%20%28double-precision%29) (ElapsedSeconds :type Float%20%28double-precision%29) (TriggeredSeconds :type Float%20%28double-precision%29) (InputAction :type Input%20Action%20Object%20Reference :default "/Game/Inputs/IA_LeftRight.IA_LeftRight"))
  (bind _returnvalue (Transformation|GetActorRotation))
  (bind _returnvalue_2 (Transformation|GetActorRotation))
  (if (< ActionValue 0.0)
    (Transformation|SetActorRotation (Math|Rotator|MakeRotator (+ (.roll _returnvalue) -0.1) (.pitch _returnvalue) 0.0))
    (else
      (Transformation|SetActorRotation (Math|Rotator|MakeRotator (+ (.roll _returnvalue_2) 0.1) (.pitch _returnvalue_2) 0.0)))))

(event Input|EnhancedActionEvents|EnhancedInputActionIA_UpDown
  (params (ActionValue :type Float%20%28double-precision%29) (ElapsedSeconds :type Float%20%28double-precision%29) (TriggeredSeconds :type Float%20%28double-precision%29) (InputAction :type Input%20Action%20Object%20Reference :default "/Game/Inputs/IA_UpDown.IA_UpDown"))
  (bind _returnvalue (Transformation|GetActorRotation))
  (bind _returnvalue_2 (Transformation|GetActorRotation))
  (if (< ActionValue 0.0)
    (Transformation|SetActorRotation (Math|Rotator|MakeRotator (.roll _returnvalue) (+ (.pitch _returnvalue) 0.1) 0.0))
    (else
      (Transformation|SetActorRotation (Math|Rotator|MakeRotator (.roll _returnvalue_2) (+ (.pitch _returnvalue_2) -0.1) 0.0)))))

(event EventBeginPlay
  (bind _asbp_my_controller (Utilities|Casting|CastToBP_MyController (Pawn|GetController)))
  (bind _output_get (Variables|Default|SetTheController _asbp_my_controller))
  (Input|AddMappingContext (PlayerController|LocalPlayerSubsystems|GetEnhancedInputLocalPlayerSubsystem _output_get) "/Game/Inputs/IMC_Inputs.IMC_Inputs" 0 "(bIgnoreAllPressedKeysUntilRelease=True,bForceImmediately=False,bNotifyUserSettings=False)")
  (CallFunction|DropBall))

(fn ConstructionScript)