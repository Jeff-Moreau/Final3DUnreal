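; Level-one actor for a ball game, pairing a ball drop point and a goal trigger with the player's BP_PawnLevelOne.
; On BeginPlay it caches the pawn as TheTable and has it drop a ball at the BallDrop location.
; A player ball overlapping Box is destroyed and triggers NextLevel on the pawn.
; Player ball hits on Base play the ball's hit sound.
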(event OnComponentBeginOverlap(Box)
  (params (OverlappedComponent :type Primitive%20Component%20Object%20Reference) (OtherActor :type Actor%20Object%20Reference) (OtherComp :type Primitive%20Component%20Object%20Reference) (OtherBodyIndex :type Integer) (bFromSweep :type Boolean) (SweepResult :type Hit%20Result%20Structure%20%28by%20ref%29))
  (bind _asbp_player_ball (Utilities|Casting|CastToBP_PlayerBall OtherActor))
  (Actor|DestroyActor _asbp_player_ball)
  (Development|PrintString "Next Level")
  (Default|NextLevel (Variables|Default|GetTheTable)))

(event OnComponentHit(Base)
  (params (HitComponent :type Primitive%20Component%20Object%20Reference) (OtherActor :type Actor%20Object%20Reference) (OtherComp :type Primitive%20Component%20Object%20Reference) (NormalImpulse :type Vector :default "0, 0, 0") (Hit :type Hit%20Result%20Structure%20%28by%20ref%29))
  (bind _asbp_player_ball (Utilities|Casting|CastToBP_PlayerBall OtherActor))
  (Default|PlayHitsound _asbp_player_ball))

(event EventBeginPlay
  (bind _asbp_pawn_level_one (Utilities|Casting|CastToBP_PawnLevelOne (Game|Player|GetPlayerPawn 0)))
  (bind _output_get (Variables|Default|SetTheTable _asbp_pawn_level_one))
  (Default|DropBall _output_get (Transformation|GetWorldLocation (Variables|Default|GetBallDrop))))

(fn ConstructionScript)